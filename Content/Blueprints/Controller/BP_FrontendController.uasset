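; BP_FrontendController is the player controller for the frontend menus, setting up the root UI layout and first screen.
; On BeginPlay it registers the default input mapping context with Enhanced Input user settings.
; When the loading screen deactivates, it creates the primary layout widget, registers it with the Frontend UI subsystem, and pushes the tag-resolved Press Any Key soft widget class onto the frontend widget stack.
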(event EventBeginPlay
  (CallFunction|RegisterInputs))

(event EventOnLoadingScreenDeactivated
  (bind _returnvalue (UserInterface|CreateWidget "/Game/Blueprints/Widgets/WBP_CUW_PrimaryLayout.WBP_CUW_PrimaryLayout_C" self))
  (UserInterface|Viewport|AddtoViewport _returnvalue 0)
  (Class|FrontendUISubsystem|RegisterCreatedPrimaryLayoutWidget (Subsystems|GetFrontendUISubsystem) _returnvalue)
  (|PushSoftWidget self (Class|FrontendFunctionLibrary|GetFrontendSoftWidgetClassbyTag "(TagName=\"Frontend.Widget.PressAnyKeyScreen\")") "(TagName=\"Frontend.WidgetStack.Frontend\")" true))

(fn ConstructionScript)

(fn RegisterInputs
  (Class|EnhancedInputUserSettings|RegisterInputMappingContext (Class|EnhancedInputSubsystemInterface|GetUserSettings (PlayerController|LocalPlayerSubsystems|GetEnhancedInputLocalPlayerSubsystem)) "/Game/Blueprints/Inputs/IMC_Default.IMC_Default"))